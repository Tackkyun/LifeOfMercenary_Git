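; BP_MainSceneOwner is a main-scene actor that opens the store UI after being tapped.
; BeginPlay creates UI_Store with its Inventory and registers it as "Store" in the HUD manager.
; Releasing a touch on BoxCollision binds CameraMoveExit to the main scene camera.
; That callback restores query collision when Begin is true; otherwise, if camera tick is off, it draws the store and disables collision.
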(event OnInputTouchEnd(boxCollision)
  (params (FingerIndex :type ETouchIndex%20Enum :default "Touch1") (TouchedComponent :type Primitive%20Component%20Object%20Reference))
  (bind _returnvalue (Class|LoMFunctions|GetMainSceneCamera))
  (EventDispatchers|BindEventtoCameraMoveExit _returnvalue (delegate Custom|CameraMoveExit)))

(event Custom|CameraMoveExit
  (params (_begin :type Boolean))
  (if _begin
    (Collision|SetCollisionEnabled (Variables|Default|GetboxCollision) "QueryOnly")
    (else
      (bind _returnvalue (Class|LoMFunctions|GetMainSceneCamera))
      (if (not (Class|Actor|IsActorTickEnabled _returnvalue))
        (bind _returnvalue_2 (Class|LoMFunctions|GetHUDManager))
        (Class|HUDManager|DrawUI _returnvalue_2 "Store")
        (Collision|SetCollisionEnabled (Variables|Default|GetboxCollision) "NoCollision")))))

(event EventBeginPlay
  (bind _returnvalue (UserInterface|CreateWidget "/Game/UI/UI_Store.UI_Store_C" 0 (Variables|Default|GetInventory)))
  (UserInterface|Viewport|AddtoViewport _returnvalue 0)
  (bind _returnvalue_2 (Class|LoMFunctions|GetHUDManager))
  (Class|HUDManager|AddUI _returnvalue_2 _returnvalue "Store"))

(event Collision|EventActorBeginOverlap
  (params (OtherActor :type Actor%20Object%20Reference)))

(event EventTick
  (params (DeltaSeconds :type Float%20%28single-precision%29)))

(fn ConstructionScript)