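; BP_MapPoint is a tappable point actor in the map scene that opens the UI_MapPoint screen for itself.
; When a touch ends on its Sphere, it checks IsTouchMove on BP_MapScenePlayerController to ignore touch-move gestures.
; Otherwise it finds UI_MapPoint through the HUD manager, passes itself in and draws it.
; An unconnected branch that would move MapCharacter to this point never runs.
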(event OnInputTouchEnd(Sphere)
  (params (FingerIndex :type ETouchIndex%20Enum :default "Touch1") (TouchedComponent :type Primitive%20Component%20Object%20Reference))
  (bind _asbp_map_scene_player_controller (Utilities|Casting|CastToBP_MapScenePlayerController (Game|GetPlayerController 0)))
  (if (not (Variables|/Game/GameMode/BP_MapScenePlayerController.BP_MapScenePlayerController_C|GetisTouchMove _asbp_map_scene_player_controller))
    (bind _returnvalue (Class|LoMFunctions|GetHUDManager))
    (bind _returnvalue_2 (Class|HUDManager|FindUI _returnvalue "UI_MapPoint"))
    (bind _asui_map_point (Utilities|Casting|CastToUI_MapPoint _returnvalue_2))
    (Default|SetMapPointUI _asui_map_point self)
    (Class|HUDManager|DrawUI _returnvalue "UI_MapPoint")))

(event EventBeginPlay)

(event Collision|EventActorBeginOverlap
  (params (OtherActor :type Actor%20Object%20Reference)))

(event EventTick
  (params (DeltaSeconds :type Float%20%28single-precision%29)))

(fn ConstructionScript)