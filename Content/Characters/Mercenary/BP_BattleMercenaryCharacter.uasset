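; Battle-mode mercenary character that shows the battle HUD, deals melee damage and rotates the camera by touch.
; BeginPlay registers the UI_Battle widget with the HUD manager and draws it.
; On damage it enters the Damage state and uses dot products to set side hit-reaction flags in the AnimBP, otherwise changing walk speed.
; An attack collision box applies damage once per enable, and touch drags yaw the camera, with release ending a block.
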(event OnComponentBeginOverlap(AttackCollisionBox)
  (params (OverlappedComponent :type Primitive%20Component%20Object%20Reference) (OtherActor :type Actor%20Object%20Reference) (OtherComp :type Primitive%20Component%20Object%20Reference) (OtherBodyIndex :type Integer) (bFromSweep :type Boolean) (SweepResult :type Hit%20Result%20Structure%20%28by%20ref%29))
  (if (Variables|Default|GetbAttackEnable)
    (Game|Damage|ApplyDamage OtherActor 1e+02 0 0)
    (Variables|Default|SetbAttackEnable false)
    (Development|PrintString "Hello")))

(event EventBeginPlay
  (bind _returnvalue (UserInterface|CreateWidget "/Game/UI/Battle/UI_Battle.UI_Battle_C" 0 self))
  (UserInterface|Viewport|AddtoViewport _returnvalue 0)
  (bind _returnvalue_2 (Class|LoMFunctions|GetHUDManager))
  (Class|HUDManager|AddUI _returnvalue_2 _returnvalue "Battle")
  (Class|HUDManager|DrawUI _returnvalue_2 "Battle"))

(event Game|Damage|EventAnyDamage
  (params (Damage :type Float%20%28single-precision%29) (DamageType :type Damage%20Type%20Object%20Reference) (InstigatedBy :type Controller%20Object%20Reference) (DamageCauser :type Actor%20Object%20Reference))
  (Variables|Default|SetcurrentState "Damage")
  ;[1 1 1] 피격위치 얻어오기
  (bind _asabp_battle_mercenary (Utilities|Casting|CastToABP_BattleMercenary (Components|SkeletalMesh|GetAnimInstance (Variables|Character|GetMesh))))
  (bind _output_get (Variables|Default|SetdamageDirection (Math|Vector|Normalize (- (Transformation|GetActorLocation) (Transformation|GetActorLocation DamageCauser)))))
  (if (>= (Math|Vector|DotProduct _output_get (Transformation|GetActorRightVector)) 0.7)
    (Variables|/Game/Characters/Mercenary/Animation/ABP_BattleMercenary.ABP_BattleMercenary_C|SetCheck_FB_LR _asabp_battle_mercenary true)
    (Variables|/Game/Characters/Mercenary/Animation/ABP_BattleMercenary.ABP_BattleMercenary_C|SetCheck_LR _asabp_battle_mercenary 1.0)
    (elif (<= (Math|Vector|DotProduct _output_get (Transformation|GetActorRightVector)) -0.7)
      (Variables|/Game/Characters/Mercenary/Animation/ABP_BattleMercenary.ABP_BattleMercenary_C|SetCheck_FB_LR _asabp_battle_mercenary true)
      (Variables|/Game/Characters/Mercenary/Animation/ABP_BattleMercenary.ABP_BattleMercenary_C|SetCheck_LR _asabp_battle_mercenary -1.0)
      (else
        (Variables|/Game/Characters/Mercenary/Animation/ABP_BattleMercenary.ABP_BattleMercenary_C|SetCheck_FB_LR _asabp_battle_mercenary false)
        (Variables|/Script/Engine.CharacterMovementComponent|SetMaxWalkSpeed (Variables|Character|GetCharacterMovement) 2e+02)))))

(event Input|TouchEvents|InputTouch
  (params (Location :type Vector) (FingerIndex :type ETouchIndex%20Enum))
  (bind _x (Math|Vector|BreakVector Location))
  ;[1 1 1] 카메라 회전 관련
  (:Pressed
    (Variables|Default|SetOrgTouchXPoint _x))
  (:Released
    (Variables|Default|SetbCameraRotEnable true)
    (if (Utilities|Enum|Equal(Enum) (Variables|Default|GetcurrentState) "Block")
      (Class|BattleMercenaryCharacter|UnBlock)))
  (:Moved
    (if (Variables|Default|GetbCameraRotEnable)
      (Pawn|Input|AddControllerYawInput (/ (- (Variables|Default|GetOrgTouchXPoint) _x) (Variables|Default|GetcameraRotSpeed)))
      (Variables|Default|SetOrgTouchXPoint _x))))

(fn ConstructionScript)